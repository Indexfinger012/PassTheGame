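; BP_Target is a hittable target that lights up and reports its order number to a manager, apparently as part of an input-order sequence.
; Each hit on its Sphere sends OrderNum to the Manager, even if already lit, then turns the target on if it is off.
; TurnOn and TurnOff events switch the PointLight intensity and the TurnedOn flag, which starts off at BeginPlay.
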(event `self.ReceiveBeginPlay`
  (`LightComponent.SetIntensity` (`self.PointLight`) 0.0)
  (set `self.TurnedOn` false))

(event `self.Sphere.OnComponentHit`
  (params (HitComponent :type "PrimitiveComponent Object Reference") (OtherActor :type "Actor Object Reference") (OtherComp :type "PrimitiveComponent Object Reference") (NormalImpulse :type "Vector Structure") (Hit :type "HitResult Structure (by ref)"))
  (`/Game/Blueprints/BP_TargetSpawn.SetInputOrder` (`self.Manager`) (`self.OrderNum`))
  (if (not (`self.TurnedOn`))
    (`self.TurnOn`)))

(event `TurnOn`
  (`LightComponent.SetIntensity` (`self.PointLight`) 2500.0)
  (set `self.TurnedOn` true))

(event `TurnOff`
  (`LightComponent.SetIntensity` (`self.PointLight`) 0.0)
  (set `self.TurnedOn` false))

(fn `UserConstructionScript`)