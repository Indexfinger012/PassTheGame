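; Enemy spawner actor that endlessly spawns Bp_enemy at its own root transform until the player reaches the kill target.
; BeginPlay runs a Delay-based loop that spawns an enemy regardless of collision, gives it a default controller, then checks EnemyKills on BP_FirstPersonCharacter.
; When that count equals exactly 50 at a check, it opens L_Tutorial; a failed player cast stops the loop.
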(event `self.ReceiveBeginPlay`
  (`KismetSystemLibrary.Delay` 1.5 :!label _label)
  (bind _returnvalue (`|SpawnActorFromClass` "/Game/Blueprints/bp_enemy.bp_enemy_C" (`SceneComponent.K2_GetComponentToWorld` (`self.DefaultSceneRoot`)) "AlwaysSpawn" "MultiplyWithRoot" null null))
  (`Pawn.SpawnDefaultController` _returnvalue)
  (`KismetSystemLibrary.Delay` 1.5)
  (bind _asbp_first_person_character (cast `/Game/FirstPerson/Blueprints/BP_FirstPersonCharacter` (`GameplayStatics.GetPlayerCharacter` 0)))
  (if (== (`/Game/FirstPerson/Blueprints/BP_FirstPersonCharacter.EnemyKills` _asbp_first_person_character) 50)
    (`GameplayStatics.OpenLevel` "L_Tutorial")
    (else
      (goto _label))))

(fn `UserConstructionScript`)