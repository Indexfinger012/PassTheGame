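; BP_PuzzleController sequences a puzzle made of BP_TargetSpawn walls, activating them one at a time.
; On BeginPlay it orders the spawns by WallOrder with a nested scan, then starts the first pattern after a short delay.
; Each WallComplete event advances to the next wall; after the last, it plays a congratulation sound, waits, then makes BP_PuzzleLevelTeleport reappear and flags it done.
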(event `self.ReceiveBeginPlay`
  (set `self.Sniffer` 0)
  (bind _outactors (`GameplayStatics.GetAllActorsOfClass` "/Game/Blueprints/BP_TargetSpawn.BP_TargetSpawn_C"))
  (for _ (range (`KismetArrayLibrary.Array_Length` _outactors))
    (for _array_element _outactors
      (if (== (`/Game/Blueprints/BP_TargetSpawn.WallOrder` _array_element) (`self.Sniffer`))
        (`KismetArrayLibrary.Array_Add` (`self.TargetSpawnOrder`) _array_element)))
    (bind _output_get (set `self.Sniffer` (+ (`self.Sniffer`) 1)))
    (`KismetSystemLibrary.PrintString` (`KismetStringLibrary.Conv_IntToString` _output_get) true true (struct :`G` 0.66 :`B` 1.0 :`A` 1.0) 5.0))
  (`KismetSystemLibrary.Delay` 5.0)
  (`self.StartOne`))

(event `StartOne`
  (bind _activetargetspawn (`self.ActiveTargetSpawn`))
  (`KismetSystemLibrary.PrintString` (`KismetStringLibrary.Conv_IntToString` _activetargetspawn))
  (`/Game/Blueprints/BP_TargetSpawn.ShowPattern` (`|GetArrayItem` (`self.TargetSpawnOrder`) _activetargetspawn)))

(event `WallComplete`
  (bind _output_get (set `self.ActiveTargetSpawn` (+ (`self.ActiveTargetSpawn`) 1)))
  (`KismetSystemLibrary.Delay` 5.0)
  (if (`KismetArrayLibrary.Array_IsValidIndex` (`self.TargetSpawnOrder`) _output_get)
    (`self.StartOne`)
    (else
      (bind _returnvalue (`GameplayStatics.GetActorOfClass` "/Game/Blueprints/BP_PuzzleLevelTeleport.BP_PuzzleLevelTeleport_C"))
      (`GameplayStatics.PlaySound2D` "/Game/LevelPrototyping/Audio/CongratsIGuess.CongratsIGuess" 1.0 1.0 0.0 null null)
      (`KismetSystemLibrary.Delay` 45.0)
      (`/Game/Blueprints/BP_PuzzleLevelTeleport.REAPPEAR` _returnvalue)
      (set `/Game/Blueprints/BP_PuzzleLevelTeleport.WeDoneHere` true _returnvalue))))

(fn `UserConstructionScript`)