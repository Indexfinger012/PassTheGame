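; Enemy Blueprint that chases the player, takes damage and restarts the level on contact.
; It repeatedly runs AI MoveTo toward the player character, retrying after a short delay whether the move succeeds or fails.
; At zero health it fires a particle event, increments the first-person character's kill count, plays a sound and destroys itself.
; Overlap of its Damge component with a player-tagged actor reloads the current level.
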(event `self.ReceiveBeginPlay`
  (`|AIMoveTo` self (0.0 0.0 0.0) (`GameplayStatics.GetPlayerCharacter` 0) :!label _label
    (:`OnSuccess`
      _)
    (:`OnFail`
      _))
  (`KismetSystemLibrary.Delay` 1.0)
  (goto _label))

(event `self.ReceiveAnyDamage`
  (params (Damage :type "Float (single-precision)") (DamageType :type "DamageType Object Reference") (InstigatedBy :type "Controller Object Reference") (DamageCauser :type "Actor Object Reference"))
  (set `self.health` (- (`self.health`) Damage))
  (if (<= (`self.health`) 0.0)
    (`ParticleSystemComponent.GenerateParticleEvent` (`self.P_Explosion`) "None" 0.0 (`self.K2_GetActorLocation`) (0.0 0.0 0.0) (0.0 0.0 0.0))
    (`|ExecutionSequence`
      (:`then_0`
        (bind _asbp_first_person_character (cast `/Game/FirstPerson/Blueprints/BP_FirstPersonCharacter` (`GameplayStatics.GetPlayerCharacter` 0)))
        (`/Engine/EditorBlueprintResources/StandardMacros.IncrementInt` (`/Game/FirstPerson/Blueprints/BP_FirstPersonCharacter.EnemyKills` _asbp_first_person_character)))
      (:`then_1`
        (`GameplayStatics.PlaySound2D` "/Engine/VREditor/Sounds/VR_click1_Cue.VR_click1_Cue" 1.0 1.0 0.0 null null)
        (`self.K2_DestroyActor`)))))

(event `self.damge.OnComponentBeginOverlap`
  (params (OverlappedComponent :type "PrimitiveComponent Object Reference") (OtherActor :type "Actor Object Reference") (OtherComp :type "PrimitiveComponent Object Reference") (OtherBodyIndex :type Integer) (bFromSweep :type Boolean) (SweepResult :type "HitResult Structure (by ref)"))
  (if (`self.ActorHasTag` OtherActor "player")
    (bind _returnvalue (`GameplayStatics.GetCurrentLevelName` true))
    (`GameplayStatics.OpenLevel` (`KismetStringLibrary.Conv_StringToName` _returnvalue))))

(fn `UserConstructionScript`)