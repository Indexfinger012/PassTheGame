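; Target spawner and manager for a memory-sequence puzzle that reports completion to BP_PuzzleController.
; BeginPlay spawns HowMany+1 indexed targets at random Y/Z offsets around itself.
; ShowPattern waits, lights targets one by one in index order, then switches them off.
; SetInputOrder collects hits; CheckInput compares the full sequence, calling WallComplete on success or printing an insult, resetting and replaying on failure.
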(event `self.ReceiveBeginPlay`
  (for _index (range (+ (`self.HowMany`) 1))
    (bind _returnvalue (`|SpawnActorFromClass` "/Game/Blueprints/BP_Target.BP_Target_C" (`KismetMathLibrary.MakeTransform` (`KismetMathLibrary.MakeVector` (.x (.location (`self.GetTransform`))) (+ (.y (.location (`self.GetTransform`))) (`KismetMathLibrary.RandomFloatInRange` -1000.0 1000.0)) (+ (.z (.location (`self.GetTransform`))) (`KismetMathLibrary.RandomFloatInRange` -200.0 200.0))) (.rotation (`self.GetTransform`)) (.scale (`self.GetTransform`))) "Undefined" "MultiplyWithRoot" null null))
    (set `/Game/Blueprints/BP_Target.OrderNum` _index _returnvalue)
    (set `/Game/Blueprints/BP_Target.Manager` self _returnvalue)
    (`KismetArrayLibrary.Array_Add` (`self.Targets`) _returnvalue)))

(event `ShowPattern`
  (bind _howmany (`self.HowMany`))
  (bind _targets (`self.Targets`))
  (`KismetSystemLibrary.Delay` 5.0)
  (bind _index (`/Game/Blueprints/TheMacroLibrary.ForLoopWithDelay` 0 _howmany 1.0)
    (:`Loop Body`
      (`/Game/Blueprints/BP_Target.TurnOn` (`|GetArrayItem` _targets _index)))
    (:`Completed`
      (for _index_2 (range (+ _howmany 1))
        (`/Game/Blueprints/BP_Target.TurnOff` (`|GetArrayItem` _targets _index_2))))))

(event `SetInputOrder`
  (params (HitTarget :type Integer))
  (bind _inputorder (`self.InputOrder`))
  (`KismetArrayLibrary.Array_Add` _inputorder HitTarget)
  (if (== (`KismetArrayLibrary.Array_Length` _inputorder) (+ 1 (`self.HowMany`)))
    (`self.CheckInput`)))

(event `CheckInput`
  (bind _howmany (`self.HowMany`))
  (for _index (range (+ _howmany 1))
    (if (== _index (`|GetArrayItem` (`self.InputOrder`) _index))
      (set `self.HasCorrectOrder` true)
      (else
        (set `self.HasCorrectOrder` false)
        (break))))
  (if (`self.HasCorrectOrder`)
    (`KismetSystemLibrary.PrintString` "NICE JOB")
    (bind _returnvalue (`GameplayStatics.GetActorOfClass` "/Game/Blueprints/BP_PuzzleController.BP_PuzzleController_C"))
    (`/Game/Blueprints/BP_PuzzleController.WallComplete` _returnvalue)
    (else
      (`KismetSystemLibrary.PrintString` "YOU FUCKIN LOSER YOU SUCK YOU\"LL NEVER HAVE FRIENDS BECAUSE YOU CAN\"T EVEN MEMORIZE A STUPID PATTERN")
      (`KismetSystemLibrary.Delay` 0.5)
      (for _index_2 (range (+ _howmany 1))
        (`/Game/Blueprints/BP_Target.TurnOff` (`|GetArrayItem` (`self.Targets`) _index_2)))
      (`KismetSystemLibrary.Delay` 2.0)
      (`KismetArrayLibrary.Array_Clear` (`self.InputOrder`))
      (`self.ShowPattern`))))

(fn `UserConstructionScript`)